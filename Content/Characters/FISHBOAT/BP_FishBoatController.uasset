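; BP_FishBoatController is the controller for the fish boat character, handling look input.
; The IA_Look Enhanced Input action calls AddLookInput, which feeds the action's X and Y into controller yaw and pitch, then prints the value to screen.
; StoreEssentialVariables caches the controlled Character and its movement component, but nothing in this Blueprint calls it.
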(event `EnhancedInput|/Game/Characters/FISHBOAT/Input/IA_Look`
  (params (ActionValue :type "Vector2D Structure") (ElapsedSeconds :type "Float (double-precision)") (TriggeredSeconds :type "Float (double-precision)") (InputAction :type "InputAction Object Reference" :default "/Game/Characters/FISHBOAT/Input/IA_Look.IA_Look"))
  (:`Triggered`
    (`self.AddLookInput`)
    (`KismetSystemLibrary.PrintString` (`KismetStringLibrary.Conv_Vector2dToString` ActionValue))))

(fn `AddLookInput`
  (bind (_returnvalue_x _returnvalue_y) (`KismetMathLibrary.BreakVector2D` (`|GetInputActionValue`)))
  (`self.AddYawInput` _returnvalue_x)
  (`self.AddPitchInput` _returnvalue_y))

(fn `StoreEssentialVariables`
  (bind _ascharacter (cast `Character` (`self.K2_GetPawn`)))
  (set `self.As Character` _ascharacter)
  (bind _ascharacter_movement_component (cast `CharacterMovementComponent` (`Pawn.GetMovementComponent` (`self.K2_GetPawn`))))
  (set `self.As Character Movement Component` _ascharacter_movement_component))

(fn `UserConstructionScript`)