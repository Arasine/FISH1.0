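; BP_FISHBOATPAWN is a fishing boat pawn driven by W, A and D debug keys.
; W repeatedly applies a forward impulse to the FishingBoat component, while A and D turn the actor by interpolating yaw left or right.
; Each key sets a held flag that sustains a short Delay loop instead of using Tick.
; The IA_Look input event is an empty stub.
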(event Input|EnhancedActionEvents|EnhancedInputActionIA_Look
  (params (ActionValue :type Vector%202D%20Structure) (ElapsedSeconds :type Float%20%28double-precision%29) (TriggeredSeconds :type Float%20%28double-precision%29) (InputAction :type Input%20Action%20Object%20Reference :default "/Game/Characters/FISHBOAT/Input/IA_Look.IA_Look")))

(event EventBeginPlay)

(event Collision|EventActorBeginOverlap
  (params (OtherActor :type Actor%20Object%20Reference)))

(event Input|KeyboardEvents|DebugKeyW
  (params (Key :type Key%20Structure :default "None") (ActionValue :type Input%20Action%20Value%20Structure))
  (:Pressed
    (Variables|Default|SetWPressed true)
    (if (Variables|Default|GetWPressed) :!label _label
      (Physics|AddImpulse (Variables|Default|Getfishing_boat) (* (Transformation|GetActorForwardVector) 8e+03) "None" false)
      (Utilities|FlowControl|Delay 0.05)
      (goto _label)))
  (:Released
    (Variables|Default|SetWPressed false)
    (goto _label)))

(event Input|KeyboardEvents|DebugKeyA
  (params (Key :type Key%20Structure :default "None") (ActionValue :type Input%20Action%20Value%20Structure))
  (bind _returnvalue (Transformation|GetActorRotation))
  (:Pressed
    (Variables|Default|SetApressed true)
    (if (Variables|Default|GetApressed) :!label _label
      (Transformation|SetActorRotation (Math|Rotator|MakeRotator 0.0 0.0 (.yaw (Math|Interpolation|RInterpTo (Math|Rotator|MakeRotator 0.0 0.0 (.yaw _returnvalue)) (Math|Rotator|MakeRotator 0.0 0.0 (- (.yaw _returnvalue) 5e+01)) (Utilities|Time|GetWorldDeltaSeconds) 6.0))))
      (Utilities|FlowControl|Delay 0.05)
      (goto _label)))
  (:Released
    (Variables|Default|SetApressed false)
    (goto _label)))

(event Input|KeyboardEvents|DebugKeyD
  (params (Key :type Key%20Structure :default "None") (ActionValue :type Input%20Action%20Value%20Structure))
  (bind _returnvalue (Transformation|GetActorRotation))
  (:Pressed
    (Variables|Default|SetDPressed true)
    (if (Variables|Default|GetDPressed) :!label _label
      (Transformation|SetActorRotation (Math|Rotator|MakeRotator 0.0 0.0 (.yaw (Math|Interpolation|RInterpTo (Math|Rotator|MakeRotator 0.0 0.0 (.yaw _returnvalue)) (Math|Rotator|MakeRotator 0.0 0.0 (+ (.yaw _returnvalue) 5e+01)) (Utilities|Time|GetWorldDeltaSeconds) 6.0))))
      (Utilities|FlowControl|Delay 0.05)
      (goto _label)))
  (:Released
    (Variables|Default|SetDPressed false)
    (goto _label)))

(fn ConstructionScript)